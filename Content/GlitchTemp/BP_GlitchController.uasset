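; Glitch effect controller that drives the MPC_GlitchV material parameter collection between Start and Stop events.
; A delay loop starts randomized bursts, switching the glitch on briefly and off until the next cycle.
; While active, Tick fades burst strength and randomizes slide shift every frame.
; Block scroll parameters update only every few frames, using accumulated time horizontally and random values vertically.
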(event `Start_Event`
  (if (not (`self.IsOn`))
    (set `self.IsOn` true)
    (set `self.TimerBlock` 0.0)
    (set `self.FrameCounterBlock` 0)
    (`self.SetDynamicParams` :!label _label)
    (`KismetSystemLibrary.Delay` (`self.GlitchTimeScan`))
    (`KismetMaterialLibrary.SetScalarParameterValue` "/ShaderLibrary/GlitchTemp/MPC_GlitchV.MPC_GlitchV" "GlitchSwitch")
    (`KismetSystemLibrary.Delay` (- (`self.WaitTimeScan`) (`self.GlitchTimeScan`)))
    (if (`self.IsOn`)
      (goto _label))))

(event `self.ReceiveTick`
  (params (DeltaSeconds :type "Float (single-precision)"))
  (if (`self.IsOn`)
    (`|ExecutionSequence`
      (:`then_0`
        (`self.UpdateParams` DeltaSeconds))
      (:`then_1`
        (set `self.TimerBlock` (+ DeltaSeconds (`self.TimerBlock`)))
        (bind _output_get (set `self.FrameCounterBlock` (+ (`self.FrameCounterBlock`) 1)))
        (if (== (mod _output_get (`self.SkipFrameBlock`)) 0)
          (`KismetMaterialLibrary.SetScalarParameterValue` "/ShaderLibrary/GlitchTemp/MPC_GlitchV.MPC_GlitchV" "HScroll" (`self.TimerBlock`))
          (`KismetMaterialLibrary.SetScalarParameterValue` "/ShaderLibrary/GlitchTemp/MPC_GlitchV.MPC_GlitchV" "VScroll" (`KismetMathLibrary.RandomFloatInRange` 0.0 1.0)))))))

(event `Stop_Event`
  (set `self.IsOn` false))

(fn `SetDynamicParams`
  (set `self.WaitTimeScan` (`KismetMathLibrary.RandomFloatInRange` 2.0 2.6))
  (set `self.GlitchTimeScan` (`KismetMathLibrary.RandomFloatInRange` 0.3 0.5))
  (set `self.StrengthScan` (`KismetMathLibrary.RandomFloatInRange` 0.002 0.004))
  (set `self.TimerScan` 0.0)
  (`KismetMaterialLibrary.SetScalarParameterValue` "/ShaderLibrary/GlitchTemp/MPC_GlitchV.MPC_GlitchV" "GlitchSwitch" 1.0))

(fn `UpdateParams`
  (params (DeltaTime :type "Float (double-precision)"))
  (`KismetMaterialLibrary.SetScalarParameterValue` "/ShaderLibrary/GlitchTemp/MPC_GlitchV.MPC_GlitchV" "GlitchStrength" (* (- 1.0 (`KismetMathLibrary.FClamp` (/ (/ (`self.TimerScan`) (`self.WaitTimeScan`)) (`self.GlitchTimeScan`)))) (`self.StrengthScan`)))
  (`KismetMaterialLibrary.SetScalarParameterValue` "/ShaderLibrary/GlitchTemp/MPC_GlitchV.MPC_GlitchV" "SlideShift" (`KismetMathLibrary.RandomFloatInRange` 0.0 1.0))
  (set `self.TimerScan` (+ DeltaTime (`self.TimerScan`))))